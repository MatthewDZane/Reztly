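; BP_G2_Example is an example Blueprint for querying a G2 snapshot API, Netbox and UE4 Nautilus data over web requests.
; Response events for login, snapshot range, snapshot query, Netbox and Nautilus each forward the request to a matching parser function.
; The request-sending nodes, which use token, URL and credential variables, and a JSON field-path lookup for flow groups are unwired, so this graph never runs them.
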(event `SnapshotRangeResponse`
  (params (Request :type "VaRestRequestJSON Object Reference"))
  ;[1 1 1] Get Available Snapshots
  (`/G2APIHelper/BP_G2_API_Helper_Library.Get Available Snapshots` Request))

(event `On Login Response`
  (params (Request :type "VaRestRequestJSON Object Reference"))
  ;[1 1 1] Get Bearer Token
  (`/G2APIHelper/BP_G2_API_Helper_Library.Get Bearer Token` Request))

(event `SnapshotQueryResponse`
  (params (Request :type "VaRestRequestJSON Object Reference"))
  ;[1 1 1] Get Snapshot
  (`/G2APIHelper/BP_G2_API_Helper_Library.Get G2 Snapshot Response` Request))

(event `OnNetboxQueryResponse`
  (params (Request :type "VaRestRequestJSON Object Reference"))
  ;[1 1 1] Get Netbox Data
  (`/G2APIHelper/BP_G2_API_Helper_Library.Get Netbox Response` Request))

(event `OnNautilusDataResponse`
  (params (Request :type "VaRestRequestJSON Object Reference"))
  ;[1 1 1] Get UE4 Data
  (`/G2APIHelper/BP_G2_API_Helper_Library.Get UE4 Response` Request))

(fn `UserConstructionScript`)